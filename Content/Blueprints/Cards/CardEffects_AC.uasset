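; Actor component on the car that applies card effects, most of which alter how the car gains or loses fuel.
; BeginPlay caches the owning Car_BP.
; Each card has its own event that sets an enable flag and its tuning values on the car, covering consumption rate, crash penalties, lane-side rewards or drains, and object-hit bonuses.
; The component only writes these variables and holds no effect logic itself.
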(event `self.ReceiveBeginPlay`
  ;[1 1 1] Get Car Ref
  (bind _ascar_bp (cast `/Game/Blueprints/Car_BP` (`self.GetOwner`)))
  (set `self.Car BP Ref` _ascar_bp))

(event `Always “right” Card Effect`
  (params (`Amount of Fuel to lose For Staying On Right` :type "Float (double-precision)"))
  (bind _car_bp_ref (`self.Car BP Ref`))
  ;[1 1 1] Alaways "Right" Card Effect
  (set `/Game/Blueprints/Car_BP.Stay on right to lose Fuel Over time` true _car_bp_ref)
  (set `/Game/Blueprints/Car_BP.Amount of Fuel to lose For Staying On Right` `Amount of Fuel to lose For Staying On Right` _car_bp_ref))

(event `Sleepy Card Effect`
  (params (`Slow Fuel Usage by Amount` :type "Float (double-precision)"))
  (bind _car_bp_ref (`self.Car BP Ref`))
  ;[1 1 1] Sleepy Card Effect
  (set `/Game/Blueprints/Car_BP.Slows fuel consumption` true _car_bp_ref)
  (set `/Game/Blueprints/Car_BP.Slow Fuel Usage by Amount` `Slow Fuel Usage by Amount` _car_bp_ref))

(event `Impatient Card Effect`
  (params (`Amount To Add to decrease fuel ` :type "Float (double-precision)"))
  (bind _car_bp_ref (`self.Car BP Ref`))
  ;[1 1 1] Impatient Card Effect
  (set `/Game/Blueprints/Car_BP.Use More Fuel` true _car_bp_ref)
  (set `/Game/Blueprints/Car_BP.Amount To Add to decrease fuel ` `Amount To Add to decrease fuel ` _car_bp_ref))

(event `Odd Fixation Card Effec`
  (params (`Gain Fuel per Hitting Specific Object Amount` :type "Float (double-precision)") (`Specific Object Index` :type Integer))
  (bind _car_bp_ref (`self.Car BP Ref`))
  ;[1 1 1] Odd Fixation Card Effect
  (set `/Game/Blueprints/Car_BP.Specific Object Index` `Specific Object Index` _car_bp_ref)
  (set `/Game/Blueprints/Car_BP.Gain Fuel per Hitting Specific Object Amount` `Gain Fuel per Hitting Specific Object Amount` _car_bp_ref)
  (set `/Game/Blueprints/Car_BP.Gain Fuel per Hitting Specific Object` true _car_bp_ref))

(event `Headphone Enjoyer Card Effect`
  (params (`Amount To Decrease the consumption of Fuel` :type "Float (double-precision)"))
  (bind _car_bp_ref (`self.Car BP Ref`))
  ;[1 1 1] HeadPhone Enjoyer Card Effect
  (set `/Game/Blueprints/Car_BP.Crashing won’t reduce your fuel gauge as much` true _car_bp_ref)
  (set `/Game/Blueprints/Car_BP.Amount To Decrease the consumption of Fuel` `Amount To Decrease the consumption of Fuel` _car_bp_ref))

(event `Left-handed Card Effect`
  (params (`Amount of Fuel For Stay On Left` :type "Float (double-precision)") (`Delay Between Fuel Reward` :type "Float (double-precision)"))
  (bind _car_bp_ref (`self.Car BP Ref`))
  ;[1 1 1] Left Handed Card Effect
  (set `/Game/Blueprints/Car_BP.Amount of Fuel For Stay On Left` `Amount of Fuel For Stay On Left` _car_bp_ref)
  (set `/Game/Blueprints/Car_BP.Delay Between Fuel Reward` `Delay Between Fuel Reward` _car_bp_ref)
  (set `/Game/Blueprints/Car_BP.Stay On The Left For Fuel` true _car_bp_ref))