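; StreetLight_BP is a street light with a configurable spotlight colour and optional flicker.
; On BeginPlay it applies LightColour to the SpotLight and, if LightFlicker is enabled, starts a looping timer at DelayBetweenFlicker intervals.
; The FlickerLight event waits briefly, hides the spotlight for FlickerDuration, then shows it again.
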(event `self.ReceiveBeginPlay`
  ;[1 1 1] Set Light Colour
  (`LightComponent.SetLightColor` (`self.SpotLight`) (`KismetMathLibrary.Conv_ColorToLinearColor` (`self.LightColour`)) true)
  (if (`self.Light Flicker`)
    (`KismetSystemLibrary.K2_SetTimerDelegate` (`|CreateDelegate` :!event `Flicker Light `) (`self.Delay Between Flicker`) true)))

(event `Flicker Light`
  ;[1 1 1] Light Flicker Event
  (`KismetSystemLibrary.Delay` 0.2)
  (`SceneComponent.SetVisibility` (`self.SpotLight`) false false)
  (`KismetSystemLibrary.Delay` (`self.Flicker Duration`))
  (`SceneComponent.SetVisibility` (`self.SpotLight`) true false))

(fn `UserConstructionScript`)