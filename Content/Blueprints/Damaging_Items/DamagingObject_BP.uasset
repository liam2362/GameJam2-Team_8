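; DamagingObject_BP is a hazard pickup that penalizes a Car_BP driving into its trigger box.
; The construction script reads the DamagingObjectList_DT row for ObjectIndex to set mesh, scale, particle template and box size.
; On overlap it drains fuel, can reverse controls or delay input, plays a sound and shows the particle, then destroys itself after a delay.
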(event `self.ReceiveBeginPlay`
  ;[1 1 1] Set Info for Random Object
)

(event `self.Box.OnComponentBeginOverlap`
  (params (OverlappedComponent :type "PrimitiveComponent Object Reference") (OtherActor :type "Actor Object Reference") (OtherComp :type "PrimitiveComponent Object Reference") (OtherBodyIndex :type Integer) (bFromSweep :type Boolean) (SweepResult :type "HitResult Structure (by ref)"))
  (bind (_objectdetails_objectmesh _objectdetails_fueldamage _objectdetails_sound _objectdetails_particle _objectdetails_triggerarea _objectdetails_reversecontrols _objectdetails_reversecontrolsduration _objectdetails_delayinput _objectdetails_inputdelayduration _objectdetails_inputdelaytime) (break `/Game/Blueprints/Damaging_Items/DamagingObjectDetails_ST` (`self.ObjectDetails`)))
  ;[1 1 1] On Overlapp Damage Players Fuel Amount
  (bind _ascar_bp (cast `/Game/FirstPerson/Blueprints/Car_BP` OtherActor))
  (if _objectdetails_reversecontrols
    (`/Game/FirstPerson/Blueprints/Car_BP. Reverse Control Event` _ascar_bp _objectdetails_reversecontrolsduration))
  (set `/Game/FirstPerson/Blueprints/Car_BP.Fuel Amount` (- (`/Game/FirstPerson/Blueprints/Car_BP.Fuel Amount` _ascar_bp) _objectdetails_fueldamage) _ascar_bp)
  (if _objectdetails_delayinput
    (`/Game/FirstPerson/Blueprints/Car_BP.DelayInput` _ascar_bp _objectdetails_inputdelayduration _objectdetails_inputdelaytime))
  (`GameplayStatics.PlaySoundAtLocation` _objectdetails_sound (`self.K2_GetActorLocation`) (struct) 1.0 1.0 0.0 null null null null)
  (`SceneComponent.SetVisibility` (`self.ParticleSystem`) true false)
  (`KismetSystemLibrary.Delay` (`self.Particle Duration`))
  (`self.K2_DestroyActor`))

(fn `UserConstructionScript`
  (bind _particlesystem (`self.ParticleSystem`))
  ;[1 1 1] Set Info for Random Object
  (bind _returnvalue (`|GetDataTableRow` "/Game/Blueprints/Damaging_Items/DamagingObjectList_DT.DamagingObjectList_DT" (`KismetStringLibrary.Conv_StringToName` (`KismetStringLibrary.Conv_IntToString` (`self.ObjectIndex`))))
    (:`then`
      (bind _output_get (set `self.ObjectDetails` _returnvalue))
      (`StaticMeshComponent.SetStaticMesh` (`self.StaticMesh`) (break `/Game/Blueprints/Damaging_Items/DamagingObjectDetails_ST` _output_get))
      (`SceneComponent.SetVisibility` _particlesystem false false)
      (`ParticleSystemComponent.SetTemplate` _particlesystem (`.particle_12_C411F1C243DAB7075D6730903C7B1699` (break `/Game/Blueprints/Damaging_Items/DamagingObjectDetails_ST` _output_get)))
      (`BoxComponent.SetBoxExtent` (`self.Box`) (`.TriggerArea_17_A10DA2204EF1318FBC11C0870B73E683` (break `/Game/Blueprints/Damaging_Items/DamagingObjectDetails_ST` _output_get)) true)
      (`SceneComponent.SetWorldScale3D` (`self.StaticMesh`) (`.MeshSize_37_72AE2BF14EF9DB88A6EA2091AB86DFDB` (break `/Game/Blueprints/Damaging_Items/DamagingObjectDetails_ST` _output_get))))))